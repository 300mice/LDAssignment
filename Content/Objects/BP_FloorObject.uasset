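; BP_FloorObject is a construction-script tool actor that builds a tiled floor and matching roof grid.
; The construction script applies the configurable floor and roof materials, then nested loops over AmountX and AmountY add instanced-mesh tiles at a fixed 200-unit spacing.
; Roof instances use negated local Y offsets relative to the floor's.
; The event graph holds no active logic.
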(event EventBeginPlay)

(event Collision|EventActorBeginOverlap
  (params (OtherActor :type Actor%20Object%20Reference)))

(event EventTick
  (params (DeltaSeconds :type Float%20%28single-precision%29)))

(fn ConstructionScript
  (Rendering|Material|SetMaterial (Variables|Default|GetRoofObject) 0 (Variables|Default|GetRoofMaterial))
  (Rendering|Material|SetMaterial (Variables|Default|GetFloorObject) 0 (Variables|Default|GetFloorMaterial))
  (for _index (range 0 (Variables|Default|GetAmountX))
    (for _index_2 (range 0 (Variables|Default|GetAmountY))
      (Components|InstancedStaticMesh|AddInstance (Variables|Default|GetFloorObject) (Math|Transform|MakeTransform (Math|Vector|MakeVector (Math|Conversions|ToFloat(Integer) (* _index 200)) (Math|Conversions|ToFloat(Integer) (* _index_2 200)) 0.0) "0, 0, 0" "1.000000,1.000000,1.000000") false)
      (Components|InstancedStaticMesh|AddInstance (Variables|Default|GetRoofObject) (Math|Transform|MakeTransform (Math|Vector|MakeVector (Math|Conversions|ToFloat(Integer) (* _index 200)) (Math|Conversions|ToFloat(Integer) (* _index_2 -200)) 0.0) "0, 0, 0" "1.000000,1.000000,1.000000") false))))