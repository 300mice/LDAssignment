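; AirRoom is a box volume that acts as an air pocket, apparently in an underwater level.
; Beginning an overlap switches player 0 to Walking, and ending it switches to Flying, each with a splash sound, without checking which actor overlapped.
; Both events also swap blend weights between its own post process and the WorldProcess actor's, which is zeroed at BeginPlay.
; The construction script sizes the box from Extent.
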(event EventBeginPlay
  (bind _returnvalue (Actor|GetActorOfClass "/Game/Blueprints/WorldProcess.WorldProcess_C"))
  (bind _output_get (Variables|Default|SetWorldPP (Variables|/Game/Blueprints/WorldProcess.WorldProcess_C|GetPostProcess _returnvalue)))
  (Variables|/Script/Engine.PostProcessComponent|SetBlendWeight _output_get 0.0))

(event EventTick
  (params (DeltaSeconds :type Float%20%28single-precision%29)))

(event Collision|EventActorBeginOverlap
  (params (OtherActor :type Actor%20Object%20Reference))
  (bind _returnvalue (Game|GetPlayerCharacter 0))
  (bind _charactermovement (Variables|/Script/Engine.Character|GetCharacterMovement _returnvalue))
  (if (Utilities|IsValid _charactermovement)
    (Pawn|Components|CharacterMovement|SetMovementMode _charactermovement "MOVE_Walking" 0)
    (Variables|/Script/Engine.PostProcessComponent|SetBlendWeight (Variables|Default|GetWorldPP) 0.0)
    (Variables|/Script/Engine.PostProcessComponent|SetBlendWeight (Variables|Default|GetPostProcess) 1.0)
    (Audio|PlaySoundatLocation "/Game/Sounds/SplashWater_BW_60919.SplashWater_BW_60919" (Transformation|GetWorldLocation (Variables|/Script/Engine.Character|GetMesh (Game|GetPlayerCharacter 0))) "0, 0, 0" 1.0 1.0 0.0 0 0 0 0)))

(event Collision|EventActorEndOverlap
  (params (OtherActor :type Actor%20Object%20Reference))
  (bind _returnvalue (Game|GetPlayerCharacter 0))
  (bind _charactermovement (Variables|/Script/Engine.Character|GetCharacterMovement _returnvalue))
  (if (Utilities|IsValid _charactermovement)
    (Pawn|Components|CharacterMovement|SetMovementMode _charactermovement "MOVE_Flying" 0)
    (Variables|/Script/Engine.PostProcessComponent|SetBlendWeight (Variables|Default|GetWorldPP) 1.0)
    (Variables|/Script/Engine.PostProcessComponent|SetBlendWeight (Variables|Default|GetPostProcess) 0.0)
    (Audio|PlaySoundatLocation "/Game/Sounds/SplashWater_BW_60919.SplashWater_BW_60919" (Transformation|GetWorldLocation (Variables|/Script/Engine.Character|GetMesh (Game|GetPlayerCharacter 0))) "0, 0, 0" 1.0 1.0 0.0 0 0 0 0)))

(fn ConstructionScript
  (Components|Box|SetBoxExtent (Variables|Default|GetBox) (Variables|Default|GetExtent) true))