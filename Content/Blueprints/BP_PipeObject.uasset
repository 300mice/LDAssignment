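; BP_PipeObject is a construction-time placement actor that builds a row of rusty metal pipe pieces from a chosen static mesh.
; The construction script loops up to Amount, adding evenly spaced mesh instances along local Y.
; It also adds raised, rotated child actors, but the integer Index / 2 == 0 test limits them to indices 0 and 1.
; Light instance and point light nodes are unconnected, and the event graph has no active logic.
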(event EventBeginPlay)

(event Collision|EventActorBeginOverlap
  (params (OtherActor :type Actor%20Object%20Reference)))

(event EventTick
  (params (DeltaSeconds :type Float%20%28single-precision%29)))

(fn ConstructionScript
  (bind _object (Variables|Default|GetObject))
  (Components|StaticMesh|SetStaticMesh _object (Variables|Default|GetStaticMesh))
  (Rendering|Material|SetMaterial _object 0 "/Game/Materials/RustyMetal/M_RustyMetal.M_RustyMetal")
  (for _index (range 0 (Variables|Default|GetAmount))
    (Components|InstancedStaticMesh|AddInstance (Variables|Default|GetObject) (Math|Transform|MakeTransform (Math|Vector|MakeVector 0.0 (Math|Conversions|ToFloat(Integer) (* _index 400)) 0.0) "0, 0, 0" "1.000000,1.000000,1.000000") false)
    (if (== (/ _index 2) 0)
      (AddComponent|AddChildActorComponent false (Math|Transform|MakeTransform (Math|Vector|MakeVector 0.0 (Math|Conversions|ToFloat(Integer) (* _index 800)) 151.0) "90.000000, 0, 0" "1.000000,1.000000,1.000000")))))