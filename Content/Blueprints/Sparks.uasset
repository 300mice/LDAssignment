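; Sparks is an actor that shows a spanner tooltip to the player while their character overlaps it.
; On BeginPlay it creates its own ToolTipSpanner widget, adds it to the viewport and hides the text block by setting its opacity to zero.
; Actor begin and end overlap events check for player character 0 and toggle that text opacity to show or hide the tooltip.
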(event EventBeginPlay
  (bind _returnvalue (UserInterface|CreateWidget "/Game/UI/ToolTip-Spanner.ToolTip-Spanner_C"))
  (Variables|Default|SetSpannerUI _returnvalue)
  (UserInterface|Viewport|AddtoViewport (Variables|Default|GetSpannerUI) 0)
  (Class|TextBlock|SetOpacity (Variables|/Game/UI/ToolTip-Spanner.ToolTip-Spanner_C|GetTextBlock_31 (Variables|Default|GetSpannerUI)) 0.0))

(event EventTick
  (params (DeltaSeconds :type Float%20%28single-precision%29)))

(event Collision|EventActorBeginOverlap
  (params (OtherActor :type Actor%20Object%20Reference))
  (if (== OtherActor (Game|GetPlayerCharacter 0))
    (Class|TextBlock|SetOpacity (Variables|/Game/UI/ToolTip-Spanner.ToolTip-Spanner_C|GetTextBlock_31 (Variables|Default|GetSpannerUI)) 1.0)))

(event Collision|EventActorEndOverlap
  (params (OtherActor :type Actor%20Object%20Reference))
  (if (== OtherActor (Game|GetPlayerCharacter 0))
    (Class|TextBlock|SetOpacity (Variables|/Game/UI/ToolTip-Spanner.ToolTip-Spanner_C|GetTextBlock_31 (Variables|Default|GetSpannerUI)) 0.0)))

(fn ConstructionScript)