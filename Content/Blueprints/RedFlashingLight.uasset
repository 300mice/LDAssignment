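; A red warning light actor that flashes while the game mode's IsMachineRunningMessage check is true.
; Each Tick it advances a time accumulator scaled by pi and TimeMultiplier, then uses its sine to drive PointLight intensity.
; The same sine feeds custom primitive data on the Light component, keeping it in step with the point light.
; When the check is false, both hold fixed steady values.
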(event EventBeginPlay)

(event Collision|EventActorBeginOverlap
  (params (OtherActor :type Actor%20Object%20Reference)))

(event EventTick
  (params (DeltaSeconds :type Float%20%28single-precision%29))
  (bind _pointlight (Variables|Default|GetPointLight))
  (bind _running (Class|BPIGameMode|IsMachineRunning(Message) (Game|GetGameMode)))
  (if _running
    (bind _output_get (Variables|Default|SetWorldTime (+ (* (Math|Float|MultiplybyPi DeltaSeconds) (Variables|Default|GetTimeMultiplier)) (Variables|Default|GetWorldTime))))
    (Rendering|Components|Light|SetIntensity _pointlight (* (Math|Trig|Sin(Radians) _output_get) 8e+03))
    (Rendering|Material|SetCustomPrimitiveDataFloat (Variables|Default|GetLight) 0 (Math|Trig|Sin(Radians) _output_get))
    (else
      (Rendering|Components|Light|SetIntensity _pointlight 5e+02)
      (Rendering|Material|SetCustomPrimitiveDataFloat (Variables|Default|GetLight) 0 0.7))))

(fn ConstructionScript)