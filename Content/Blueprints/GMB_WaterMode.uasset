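; Water mode Blueprint, apparently a game mode, that runs a periodic machine cycle and exposes its running and play states through getters.
; A looping BeginPlay timer toggles the machine state.
; Starting plays rumble and alarm sounds, then after delays adds blade sounds and finally shuts the machine off, stopping the alarm and whoop.
; Tick steadily raises the whoop's pitch while running, giving a spin-up effect.
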(event EventBeginPlay
  (Utilities|Time|SetTimerbyEvent (delegate EventChangeMachineState) 2.4e+02 true)
  (Variables|Default|SetbPlay true))

(event EventChangeMachineState
  (if (Variables|Default|GetbIsMachineRunning)
    (Variables|Default|SetbIsMachineRunning false)
    (else
      (Variables|Default|SetbIsMachineRunning true)
      (Audio|PlaySoundatLocation "/Game/Sounds/DroneRumble_BW_12009.DroneRumble_BW_12009" "0, 0, 0" "0, 0, 0" 1.0 1.0 0.0 0 0 0 0)
      (bind _returnvalue (Audio|SpawnSoundatLocation "/Game/Sounds/Battle.Battle" "0, 0, 0" "0, 0, 0" 1.0 1.0 0.0 0 0))
      (Variables|Default|SetALARM _returnvalue)
      (Utilities|FlowControl|Delay 15.0)
      (Audio|SpawnSoundatLocation "/Game/Sounds/BladeStartUp.BladeStartUp" "0, 0, 0" "0, 0, 0" 1.0 1.0 0.0 0 0)
      (bind _returnvalue_2 (Audio|SpawnSoundatLocation "/Game/Sounds/WOOP.WOOP" "0, 0, 0" "0, 0, 0" 1.0 1.0 0.0 0 0))
      (Variables|Default|SetWOOP _returnvalue_2)
      (Utilities|FlowControl|Delay 3e+01)
      (Variables|Default|SetbIsMachineRunning false)
      (Audio|Components|Audio|Stop (Variables|Default|GetALARM))
      (Audio|Components|Audio|Stop (Variables|Default|GetWOOP)))))

(event EventTick
  (params (DeltaSeconds :type Float%20%28single-precision%29))
  (bind _woop (Variables|Default|GetWOOP))
  (if (Utilities|IsValid _woop)
    (if (Variables|Default|GetbIsMachineRunning)
      (Audio|Components|Audio|SetPitchMultiplier _woop (+ (Variables|/Script/Engine.AudioComponent|GetPitchMultiplier _woop) 0.002)))))

(fn ConstructionScript)

(fn GetPlay
  (return (Variables|Default|GetbPlay)))

(fn IsMachineRunning
  (return (Variables|Default|GetbIsMachineRunning)))