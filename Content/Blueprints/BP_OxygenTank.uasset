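; BP_OxygenTank is an oxygen tank actor that shows a tooltip when the player is near it.
; On BeginPlay it creates a ToolTipOxygenTank widget, adds it to the viewport and hides its text block by zeroing opacity.
; Begin and end overlap with the player character toggle that opacity and set an Overlap flag, which the file itself never reads.
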(event EventBeginPlay
  (bind _returnvalue (UserInterface|CreateWidget "/Game/UI/ToolTip-OxygenTank.ToolTip-OxygenTank_C"))
  (Variables|Default|SetButtonUI _returnvalue)
  (UserInterface|Viewport|AddtoViewport (Variables|Default|GetButtonUI) 0)
  (Class|TextBlock|SetOpacity (Variables|/Game/UI/ToolTip-OxygenTank.ToolTip-OxygenTank_C|GetTextBlock_31 (Variables|Default|GetButtonUI)) 0.0))

(event EventTick
  (params (DeltaSeconds :type Float%20%28single-precision%29)))

(event Collision|EventActorBeginOverlap
  (params (OtherActor :type Actor%20Object%20Reference))
  (if (== OtherActor (Game|GetPlayerCharacter 0))
    (Class|TextBlock|SetOpacity (Variables|/Game/UI/ToolTip-OxygenTank.ToolTip-OxygenTank_C|GetTextBlock_31 (Variables|Default|GetButtonUI)) 1.0)
    (Variables|Default|SetbOverlap true)))

(event Collision|EventActorEndOverlap
  (params (OtherActor :type Actor%20Object%20Reference))
  (if (== OtherActor (Game|GetPlayerCharacter 0))
    (Class|TextBlock|SetOpacity (Variables|/Game/UI/ToolTip-OxygenTank.ToolTip-OxygenTank_C|GetTextBlock_31 (Variables|Default|GetButtonUI)) 0.0)
    (Variables|Default|SetbOverlap false)))

(fn ConstructionScript)