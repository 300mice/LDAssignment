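; BP_Swimmer is a player character with look, move and jump controls and a toggleable flashlight that starts off.
; Movement follows the camera's forward and right vectors, and jumping is blocked while the movement component is flying.
; Tick polls the game mode's machine-running state and uses a resettable DoOnce to play one world camera shake each time the machine starts running.
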(event EventTick
  (params (DeltaSeconds :type Float%20%28single-precision%29))
  (bind _running (Class|BPIGameMode|IsMachineRunning(Message) (Game|GetGameMode)))
  (if _running
    (Utilities|FlowControl|DoOnce false :!label _label
      (:Completed
        (Camera|PlayWorldCameraShake "/Game/Blueprints/Shake.Shake_C" "0, 0,-1000.000000" 0.0 5e+03 1.0 true)))
    (else
      (goto _label Reset))))

(event EventBeginPlay
  (Rendering|Components|Light|SetIntensity (Variables|Default|GetSpotLight) 0.0))

(event Input|ActionEvents|InputActionJump
  (params (Key :type Key%20Structure :default "None"))
  (:Pressed
    (if (not (Class|NavMovementComponent|IsFlying (Variables|Character|GetCharacterMovement)))
      (Character|Jump)))
  (:Released
    (Character|StopJumping)))

(event Input|ActionEvents|InputActionFlashlight
  (params (Key :type Key%20Structure :default "None"))
  (:Pressed
    (if (Variables|Default|GetbLight)
      (Rendering|Components|Light|SetIntensity (Variables|Default|GetSpotLight) 0.0)
      (Variables|Default|SetbLight false)
      (else
        (Rendering|Components|Light|SetIntensity (Variables|Default|GetSpotLight) 1e+03)
        (Variables|Default|SetbLight true)))))

(event Input|AxisEvents|InputAxisLookRight
  (params (AxisValue :type Float%20%28single-precision%29))
  (Pawn|Input|AddControllerYawInput AxisValue))

(event Input|AxisEvents|InputAxisLookUp
  (params (AxisValue :type Float%20%28single-precision%29))
  (Pawn|Input|AddControllerPitchInput AxisValue))

(event Input|AxisEvents|InputAxisMoveForward
  (params (AxisValue :type Float%20%28single-precision%29))
  (Pawn|Input|AddMovementInput (Math|Vector|GetForwardVector (Variables|Default|GetCamera)) AxisValue false))

(event Input|AxisEvents|InputAxisMoveRight
  (params (AxisValue :type Float%20%28single-precision%29))
  (Pawn|Input|AddMovementInput (Math|Vector|GetRightVector (Variables|Default|GetCamera)) AxisValue false))

(fn ConstructionScript)