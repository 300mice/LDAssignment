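; BigButton is an interactable actor that lets the player trigger a machine state change with the E key.
; It creates a ToolTipButton widget on BeginPlay and shows or hides its text through opacity as the player character enters or leaves the overlap.
; While overlapping, Tick polls the player controller for an E press and calls ChangeMachineStateMessage on the game mode.
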(event EventBeginPlay
  (bind _returnvalue (UserInterface|CreateWidget "/Game/UI/ToolTip-Button.ToolTip-Button_C"))
  (Variables|Default|SetButtonUI _returnvalue)
  (UserInterface|Viewport|AddtoViewport (Variables|Default|GetButtonUI) 0)
  (Class|TextBlock|SetOpacity (Variables|/Game/UI/ToolTip-Button.ToolTip-Button_C|GetTextBlock_31 (Variables|Default|GetButtonUI)) 0.0))

(event EventTick
  (params (DeltaSeconds :type Float%20%28single-precision%29))
  (if (Variables|Default|GetbOverlap)
    (if (Game|Player|WasInputKeyJustPressed (Game|GetPlayerController 0) "E")
      (Class|BPIGameMode|ChangeMachineState(Message) (Game|GetGameMode)))))

(event Collision|EventActorBeginOverlap
  (params (OtherActor :type Actor%20Object%20Reference))
  (if (== OtherActor (Game|GetPlayerCharacter 0))
    (Class|TextBlock|SetOpacity (Variables|/Game/UI/ToolTip-Button.ToolTip-Button_C|GetTextBlock_31 (Variables|Default|GetButtonUI)) 1.0)
    (Variables|Default|SetbOverlap true)))

(event Collision|EventActorEndOverlap
  (params (OtherActor :type Actor%20Object%20Reference))
  (if (== OtherActor (Game|GetPlayerCharacter 0))
    (Class|TextBlock|SetOpacity (Variables|/Game/UI/ToolTip-Button.ToolTip-Button_C|GetTextBlock_31 (Variables|Default|GetButtonUI)) 0.0)
    (Variables|Default|SetbOverlap false)))

(fn ConstructionScript)