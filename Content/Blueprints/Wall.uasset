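; Wall is a construction-time procedural Blueprint that builds a two-sided wall from instanced meshes, sized by Amount and Height.
; The construction script applies the inside material to RightWall and the outside material to LeftWall.
; Nested loops add instances to both components on a fixed-spacing grid, with LeftWall stepping in the opposite local X direction and both stepping along negative Y for each Height row.
; The event graph holds no logic.
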(event EventBeginPlay)

(event Collision|EventActorBeginOverlap
  (params (OtherActor :type Actor%20Object%20Reference)))

(event EventTick
  (params (DeltaSeconds :type Float%20%28single-precision%29)))

(fn ConstructionScript
  (Rendering|Material|SetMaterial (Variables|Default|GetRightWall) 0 (Variables|Default|GetInsideWall))
  (Rendering|Material|SetMaterial (Variables|Default|GetLeftWall) 0 (Variables|Default|GetOutsideWall))
  (for _index (range 0 (Variables|Default|GetAmount))
    (for _index_2 (range 0 (Variables|Default|GetHeight))
      (Components|InstancedStaticMesh|AddInstance (Variables|Default|GetRightWall) (Math|Transform|MakeTransform (Math|Vector|MakeVector (Math|Conversions|ToFloat(Integer) (* _index 200)) (Math|Conversions|ToFloat(Integer) (* _index_2 -200)) 0.0) "0, 0, 0" "1.000000,1.000000,1.000000") false)
      (Components|InstancedStaticMesh|AddInstance (Variables|Default|GetLeftWall) (Math|Transform|MakeTransform (Math|Vector|MakeVector (Math|Conversions|ToFloat(Integer) (* _index -200)) (Math|Conversions|ToFloat(Integer) (* _index_2 -200)) 0.0) "0, 0, 0" "1.000000,1.000000,1.000000") false))))