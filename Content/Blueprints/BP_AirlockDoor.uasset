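; Airlock door actor that closes when the game mode reports the machine is running and opens when it stops.
; Tick polls that state while the door is idle, using two DoOnce gates that re-arm each other so each change triggers one move.
; Looping timers step the door vertically, counting increments until paused, with the same door sound at each start and debug prints while moving.
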(event Custom|Open
  (bind _door (Variables|Default|GetDoor))
  (bind _returnvalue (Transformation|GetWorldLocation _door))
  (Variables|Default|SetbMoving true)
  (if (< (Variables|Default|Getint0) 180)
    (Variables|Default|Setint0 (+ (Variables|Default|Getint0) 1))
    (Transformation|SetWorldLocation (Variables|Default|GetDoor) (Math|Vector|MakeVector (.x _returnvalue) (.y _returnvalue) (+ (.z _returnvalue) 1.0)) false false)
    (Development|PrintString "Opening")
    (else
      (Variables|Default|SetbMoving false)
      (Utilities|Time|PauseTimerbyHandle (Variables|Default|GetTimedOpen)))))

(event Custom|Close
  (Variables|Default|SetbMoving true)
  (if (< (Variables|Default|Getint0) 180)
    (Variables|Default|Setint0 (+ (Variables|Default|Getint0) 1))
    (Transformation|SetRelativeLocation (Variables|Default|GetDoor) (Math|Vector|MakeVector 0.0 0.0 (+ (.z (Variables|/Script/Engine.SceneComponent|GetRelativeLocation (Variables|Default|GetDoor))) -1.0)) false false)
    (Development|PrintString "Closing")
    (else
      (Variables|Default|SetbMoving false)
      (Utilities|Time|PauseTimerbyHandle (Variables|Default|GetTimedClose)))))

(event EventBeginPlay)

(event Collision|EventActorBeginOverlap
  (params (OtherActor :type Actor%20Object%20Reference)))

(event EventTick
  (params (DeltaSeconds :type Float%20%28single-precision%29))
  (if (not (Variables|Default|GetbMoving))
    (bind _running (Class|BPIGameMode|IsMachineRunning(Message) (Game|GetGameMode)))
    (if _running
      (Utilities|FlowControl|DoOnce false :!label _label
        (:Completed
          (CallFunction|CloseAirlock)
          (goto _label_2 Reset)))
      (else
        (Utilities|FlowControl|DoOnce true :!label _label_2
          (:Completed
            (CallFunction|OpenAirlock)
            (goto _label Reset)))))))

(event EventCloseAirlock
  (Variables|Default|Setint0 0)
  (bind _returnvalue (Utilities|Time|SetTimerbyEvent (delegate Custom|Close) 0.1 true))
  (Variables|Default|SetTimedClose _returnvalue)
  (Audio|PlaySoundatLocation "/Game/Sounds/DoorClose.DoorClose" (Transformation|GetWorldLocation (Variables|Default|GetDoor)) "0, 0, 0" 1.0 1.0 0.0 0 0 0 0))

(event EventOpenAirlock
  (Variables|Default|Setint0 0)
  (bind _returnvalue (Utilities|Time|SetTimerbyEvent (delegate Custom|Open) 0.1 true))
  (Variables|Default|SetTimedOpen _returnvalue)
  (Audio|PlaySoundatLocation "/Game/Sounds/DoorClose.DoorClose" (Transformation|GetWorldLocation (Variables|Default|GetDoor)) "0, 0, 0" 1.0 1.0 0.0 0 0 0 0))

(fn ConstructionScript)